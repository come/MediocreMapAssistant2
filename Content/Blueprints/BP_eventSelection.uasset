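; Selection box actor for events on a note timeline, apparently in a beat-map editor, drawn as a stretched mesh with a selection material.
; UpdateEventSelection, also run at construction, maps event Type to a lane, scales by Width and Duration, and offsets the actor by Time using note separation.
; Negative Width mirrors the box from the lane's far edge.
; GetProperties returns Time, Line, Type and Duration as an Obstacle struct.
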(event Custom|UpdateEventSelection
  (bind _meshroot (Variables|Default|GetMeshRoot))
  (bind _meshroot_2 (Variables|Default|GetMeshRoot))
  (bind _type (Variables|Default|GetType))
  (bind _returnvalue (Utilities|Select :Index _type :Option%200 0 :Option%201 1 :Option%202 2 :Option%203 3 :Option%204 4 :Option%205 5 :Option%206 0 :Option%207 0 :Option%208 6 :Option%209 7 :Option%2010 0 :Option%2011 0 :Option%2012 8 :Option%2013 9))
  (if (>= (Variables|Default|GetWidth) 0)
    (Transformation|SetWorldScale3D _meshroot (Math|Vector|MakeVector (* (+ (Variables|Default|GetWidth) 1) 0.5) (* (Variables|Default|GetDuration) (/ (CallFunction|GetNoteSep) 1e+02)) 0.5))
    (Transformation|SetRelativeLocation _meshroot (Math|Vector|MakeVector (* _returnvalue 5e+01) 0.0 0.0) false false)
    (else
      (Transformation|SetWorldScale3D _meshroot_2 (Math|Vector|MakeVector (* (+ (Variables|Default|GetWidth) -1) 0.5) (* (Variables|Default|GetDuration) (/ (CallFunction|GetNoteSep) 1e+02)) 0.5))
      (Transformation|SetRelativeLocation _meshroot_2 (Math|Vector|MakeVector (* (+ _returnvalue 1) 5e+01) 0.0 0.0) false false)))
  (Rendering|Material|SetMaterial (Variables|Default|GetMesh) 0 "/Game/Materials/M_EventSelection.M_EventSelection")
  (Transformation|SetActorRelativeLocation (Math|Vector|MakeVector 0.0 (* (* (CallFunction|GetNoteSep) (Variables|Default|GetTime)) -1.0) 0.0)))

(fn ConstructionScript
  (CallFunction|UpdateEventSelection))

(fn GetProperties
  (return (Utilities|Struct|MakeStructObstacle (Variables|Default|GetTime) (Variables|Default|GetLine) (Variables|Default|GetType) (Variables|Default|GetDuration))))