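; BPFL_editor is a helper function library for a note-based map editor.
; Getters read shared settings from BPGI_editor: note separation, six-lane mode, precision angles and placement, and WIP.
; LineToEvent and EventToLine convert between editor lines and non-contiguous event IDs, with one large sentinel-like ID on the last line and unmapped IDs falling back to the first.
; SpawnPopup shows a message in an error popup widget at a high Z-order.
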(fn GetNoteSep
  (return (Variables|/Game/Blueprints/BPGI_editor.BPGI_editor_C|GetNoteSeparation (.AsBPGI%20Editor (Utilities|Casting|CastToBPGI_editor (Game|GetGameInstance (LocalVariables|Get__WorldContext)))))))

(fn SpawnPopup
  (params (Message :type String))
  (bind _returnvalue (UserInterface|CreateWidget "/Game/Blueprints/WidgetErrorPopup.WidgetErrorPopup_C" (Game|GetPlayerController 0) Message))
  (UserInterface|Viewport|AddtoViewport _returnvalue 10000))

(fn LinetoEvent
  (params (Line :type Integer))
  (return (Utilities|Select :Index Line :Option%200 0 :Option%201 1 :Option%202 2 :Option%203 3 :Option%204 4 :Option%205 5 :Option%206 8 :Option%207 9 :Option%208 12 :Option%209 13 :Option%2010 229818389)))

(fn EventtoLine
  (params (Event :type Integer))
  (return (select (== Event 229818389) 10 (Utilities|Select :Index Event :Option%200 0 :Option%201 1 :Option%202 2 :Option%203 3 :Option%204 4 :Option%205 5 :Option%206 0 :Option%207 0 :Option%208 6 :Option%209 7 :Option%2010 0 :Option%2011 0 :Option%2012 8 :Option%2013 9))))

(fn Get6LaneMode
  (return (Variables|/Game/Blueprints/BPGI_editor.BPGI_editor_C|Get6Lane (.AsBPGI%20Editor (Utilities|Casting|CastToBPGI_editor (Game|GetGameInstance (LocalVariables|Get__WorldContext)))))))

(fn GetPrecisionSettings
  (bind ___worldcontext (LocalVariables|Get__WorldContext))
  (bind _returnvalue (Game|GetGameInstance ___worldcontext))
  (bind _asbpgi_editor (Utilities|Casting|CastToBPGI_editor _returnvalue))
  (return (Variables|/Game/Blueprints/BPGI_editor.BPGI_editor_C|GetPrecisionAngles _asbpgi_editor) (Variables|/Game/Blueprints/BPGI_editor.BPGI_editor_C|GetPrecisionPlacement _asbpgi_editor)))

(fn GetWIP
  (return (Variables|/Game/Blueprints/BPGI_editor.BPGI_editor_C|GetWIP (.AsBPGI%20Editor (Utilities|Casting|CastToBPGI_editor (Game|GetGameInstance (LocalVariables|Get__WorldContext)))))))